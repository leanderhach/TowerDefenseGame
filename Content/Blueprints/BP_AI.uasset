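; Enemy AI pawn that heads for the first BP_DefenseHub on spawn and awards score when killed.
; Turret projectile hits subtract health by bullet type, while an attacking player knife kills instantly with a spark effect.
; Death adds difficulty-scaled points to GS_GameState, and a looping timer destroys stationary pawns without scoring.
; Also contains a tap-versus-hold HoldInput macro that the event graph never uses.
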(event OnComponentBeginOverlap(CapsuleComponent)
  (params (OverlappedComponent :type Primitive%20Component%20Object%20Reference) (OtherActor :type Actor%20Object%20Reference) (OtherComp :type Primitive%20Component%20Object%20Reference) (OtherBodyIndex :type Integer) (bFromSweep :type Boolean) (SweepResult :type Hit%20Result%20Structure%20%28by%20ref%29))
  (bind _asbp_player_knife (Utilities|Casting|CastToBP_PlayerKnife OtherActor))
  (if (Variables|/Game/Blueprints/BP_PlayerKnife.BP_PlayerKnife_C|GetisAttacking _asbp_player_knife)
    (Variables|Default|Sethealth 0)
    (Niagara|SpawnSystematLocation "/Game/Assets/Particles/hITsPARK.hitSpark" (Transformation|GetActorLocation))
    (CallFunction|AddtoPlayerScoreandKill)))

(event OnComponentHit(CapsuleComponent)
  (params (HitComponent :type Primitive%20Component%20Object%20Reference) (OtherActor :type Actor%20Object%20Reference) (OtherComp :type Primitive%20Component%20Object%20Reference) (NormalImpulse :type Vector :default "0, 0, 0") (Hit :type Hit%20Result%20Structure%20%28by%20ref%29))
  (bind _asbp_turret_projectile (Utilities|Casting|CastToBP_TurretProjectile OtherActor))
  (switch string (Variables|/Game/Blueprints/BP_TurretProjectile.BP_TurretProjectile_C|GetbulletType _asbp_turret_projectile)
    (:shortRange
      (Variables|Default|Sethealth (- (Variables|Default|Gethealth) 50)))
    (:sniper
      (Variables|Default|Sethealth (- (Variables|Default|Gethealth) 100)))
    (:playerGun
      (Variables|Default|Sethealth (- (Variables|Default|Gethealth) 25)))))

(event Custom|checkIfStationary
  (if (<= (Math|Vector|VectorLength (Transformation|GetVelocity)) 0.0)
    (Actor|DestroyActor)))

(event EventTick
  (params (DeltaSeconds :type Float%20%28single-precision%29))
  (if (<= (Variables|Default|Gethealth) 0)
    (CallFunction|AddtoPlayerScoreandKill)))

(event EventBeginPlay
  (Utilities|Time|SetTimerbyEvent (delegate Custom|checkIfStationary) 5.0 true)
  (bind _outactors (Actor|GetAllActorsOfClass "/Game/Blueprints/BP_DefenseHub.BP_DefenseHub_C"))
  (AI|AIMoveTo self (Transformation|GetActorLocation (Utilities|Array|Get(acopy) _outactors)) 0 5.0 false))

(fn ConstructionScript)

(fn AddtoPlayerScoreandKill
  (bind _asgs_game_state (Utilities|Casting|CastToGS_GameState (Game|GetGameState)))
  (Variables|/Game/Blueprints/GS_GameState.GS_GameState_C|SetplayerScore _asgs_game_state (+ (- 30 (* (Variables|/Game/Blueprints/GS_GameState.GS_GameState_C|Getdifficulty _asgs_game_state) 5)) (Variables|/Game/Blueprints/GS_GameState.GS_GameState_C|GetplayerScore _asgs_game_state)))
  (Actor|DestroyActor))