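; BP_Wall is a destructible wall that loses health when AI characters run into it.
; An overlap on ItemBounds with a BP_AI subtracts a fixed amount of WallHealth, spawns a red HitSpark Niagara effect at the AI and destroys that AI.
; Tick polls WallHealth and, once it reaches zero, spawns a blue HitSpark at the wall and destroys it.
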(event OnComponentBeginOverlap(ItemBounds)
  (params (OverlappedComponent :type Primitive%20Component%20Object%20Reference) (OtherActor :type Actor%20Object%20Reference) (OtherComp :type Primitive%20Component%20Object%20Reference) (OtherBodyIndex :type Integer) (bFromSweep :type Boolean) (SweepResult :type Hit%20Result%20Structure%20%28by%20ref%29))
  (bind _asbp_ai (Utilities|Casting|CastToBP_AI OtherActor))
  (Variables|Default|SetwallHealth (- (Variables|Default|GetwallHealth) 10))
  (bind _returnvalue (Niagara|SpawnSystematLocation "/Game/Assets/Particles/hITsPARK.hitSpark" (Transformation|GetActorLocation _asbp_ai)))
  (Niagara|SetNiagaraVariable(LinearColor) _returnvalue "sparkColor" (Utilities|Struct|MakeLinearColor 1e+03 0.0 0.0 1.0))
  (Actor|DestroyActor _asbp_ai))

(event EventTick
  (params (DeltaSeconds :type Float%20%28single-precision%29))
  (if (<= (Variables|Default|GetwallHealth) 0)
    (bind _returnvalue (Niagara|SpawnSystematLocation "/Game/Assets/Particles/hITsPARK.hitSpark" (Transformation|GetActorLocation)))
    (Niagara|SetNiagaraVariable(LinearColor) _returnvalue "sparkColor" (Utilities|Struct|MakeLinearColor 0.0 0.0 1e+03 1.0))
    (Actor|DestroyActor)))

(fn ConstructionScript)