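; Short-range defense turret that fires alternating-barrel projectiles at the first BP_AI in its RangePerimeter overlap list.
; Tick samples that target's position across PollingInterval, and TrackObject predicts an intercept point from angular and radial velocity in spherical coordinates.
; TurnTurret interpolates base yaw and barrel pitch toward that point, and a shot with sound follows FireDelay once both are within ErrorMargin.
; FireTurret is empty and TurnBarrels is never called.
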(event OnComponentEndOverlap(RangePerimeter)
  (params (OverlappedComponent :type Primitive%20Component%20Object%20Reference) (OtherActor :type Actor%20Object%20Reference) (OtherComp :type Primitive%20Component%20Object%20Reference) (OtherBodyIndex :type Integer))
  (if (> (Utilities|Array|Length (Variables|Default|GettargetsInRange)) 0)
    (Utilities|Casting|CastToBP_AI OtherActor)
    (Utilities|Array|RemoveItem (Variables|Default|GettargetsInRange) OtherActor)))

(event OnComponentBeginOverlap(RangePerimeter)
  (params (OverlappedComponent :type Primitive%20Component%20Object%20Reference) (OtherActor :type Actor%20Object%20Reference) (OtherComp :type Primitive%20Component%20Object%20Reference) (OtherBodyIndex :type Integer) (bFromSweep :type Boolean) (SweepResult :type Hit%20Result%20Structure%20%28by%20ref%29))
  (Utilities|Casting|CastToBP_AI OtherActor)
  (Utilities|Array|Add (Variables|Default|GettargetsInRange) OtherActor))

(event EventTick
  (params (DeltaSeconds :type Float%20%28single-precision%29))
  (bind _errormargin (Variables|Default|GeterrorMargin))
  (bind _fireorigin1 (Variables|Default|GetFireOrigin1))
  (bind _fireorigin2 (Variables|Default|GetFireOrigin2))
  (bind _returnvalue (Transformation|GetWorldTransform _fireorigin1))
  (bind _returnvalue_2 (Transformation|GetWorldTransform _fireorigin2))
  (if (> (Utilities|Array|Length (Variables|Default|GettargetsInRange)) 0)
    (Utilities|FlowControl|Delay 0.1)
    (Variables|Default|SetoldTargetTransform (Transformation|GetActorTransform (Utilities|Array|Get(acopy) (Variables|Default|GettargetsInRange))))
    (Utilities|FlowControl|Delay (Variables|Default|GetpollingInterval))
    (bind _enemynextposition (CallFunction|TrackObject (Variables|Default|GetoldTargetTransform) (Transformation|GetActorTransform (Utilities|Array|Get(acopy) (Variables|Default|GettargetsInRange))) (Transformation|GetActorLocation self)))
    (bind (_relative_rotation _target_rotation _relative_rotation1 _target_rotation1) (CallFunction|TurnTurret _enemynextposition))
    (if (and (Math|Rotator|Equal(Rotator) _relative_rotation _target_rotation _errormargin) (Math|Rotator|Equal(Rotator) _relative_rotation1 _target_rotation1 _errormargin))
      (Utilities|FlowControl|Delay (Variables|Default|GetfireDelay))
      (if (Variables|Default|GetturretBarrelSwitch)
        (Variables|Default|SetturretBarrelSwitch false)
        (bind _returnvalue_3 (Game|SpawnActorfromClass "/Game/Blueprints/BP_TurretProjectile.BP_TurretProjectile_C" _returnvalue "Undefined" 0 0))
        (Variables|/Game/Blueprints/BP_TurretProjectile.BP_TurretProjectile_C|SetbulletType _returnvalue_3 "shortRange")
        (Audio|PlaySoundatLocation "/Game/Assets/Audio/zapsplat_science_fiction_gunshot_powerful_blaster_001_62937.zapsplat_science_fiction_gunshot_powerful_blaster_001_62937" (.Location (Math|Transform|BreakTransform _returnvalue)) "0, 0, 0" 0.1 1.2 0.0 "/Game/Assets/Audio/BulletFireAttenuation.BulletFireAttenuation" 0 0)
        (else
          (Variables|Default|SetturretBarrelSwitch true)
          (bind _returnvalue_4 (Game|SpawnActorfromClass "/Game/Blueprints/BP_TurretProjectile.BP_TurretProjectile_C" _returnvalue_2 "Undefined" 0 0))
          (Variables|/Game/Blueprints/BP_TurretProjectile.BP_TurretProjectile_C|SetbulletType _returnvalue_4 "shortRange")
          (Audio|PlaySoundatLocation "/Game/Assets/Audio/zapsplat_science_fiction_gunshot_powerful_blaster_001_62937.zapsplat_science_fiction_gunshot_powerful_blaster_001_62937" (.Location (Math|Transform|BreakTransform _returnvalue_2)) "0, 0, 0" 0.1 1.2 0.0 "/Game/Assets/Audio/BulletFireAttenuation.BulletFireAttenuation" 0 0))))))

(fn ConstructionScript)

(fn TrackObject
  (params (InitialLocation :type Transform) (CurrentLocation :type Transform) (DefenseOrigin :type Vector))
  (bind _projectilespeed (Variables|Default|GetProjectileSpeed))
  (bind _pollinginterval (Variables|Default|GetPollingInterval))
  (Variables|Default|SetDefenseOrigin DefenseOrigin)
  (return (+ (Math|Vector|MakeVector (|(((cos(theta))*(sin(phi)))*r) (+ (Math|Trig|Atan2(Radians) (.Y (Math|Vector|BreakVector (- (.Location (Math|Transform|BreakTransform CurrentLocation)) (Variables|Default|GetDefenseOrigin)))) (.X (Math|Vector|BreakVector (- (.Location (Math|Transform|BreakTransform CurrentLocation)) (Variables|Default|GetDefenseOrigin))))) (* (/ (Math|Trig|Acos(Degrees) (/ (Math|Vector2D|DotProduct(2D) (Math|Vector2D|MakeVector2D (.X (Math|Vector|BreakVector (- (.Location (Math|Transform|BreakTransform InitialLocation)) (Variables|Default|GetDefenseOrigin)))) (.Y (Math|Vector|BreakVector (- (.Location (Math|Transform|BreakTransform InitialLocation)) (Variables|Default|GetDefenseOrigin))))) (Math|Vector2D|MakeVector2D (.X (Math|Vector|BreakVector (- (.Location (Math|Transform|BreakTransform CurrentLocation)) (Variables|Default|GetDefenseOrigin)))) (.Y (Math|Vector|BreakVector (- (.Location (Math|Transform|BreakTransform CurrentLocation)) (Variables|Default|GetDefenseOrigin)))))) (* (Math|Vector|VectorLengthXY (Math|Conversions|ToVector(Vector2D) (Math|Vector2D|MakeVector2D (.X (Math|Vector|BreakVector (- (.Location (Math|Transform|BreakTransform InitialLocation)) (Variables|Default|GetDefenseOrigin)))) (.Y (Math|Vector|BreakVector (- (.Location (Math|Transform|BreakTransform InitialLocation)) (Variables|Default|GetDefenseOrigin))))))) (Math|Vector|VectorLengthXY (Math|Conversions|ToVector(Vector2D) (Math|Vector2D|MakeVector2D (.X (Math|Vector|BreakVector (- (.Location (Math|Transform|BreakTransform CurrentLocation)) (Variables|Default|GetDefenseOrigin)))) (.Y (Math|Vector|BreakVector (- (.Location (Math|Transform|BreakTransform CurrentLocation)) (Variables|Default|GetDefenseOrigin)))))))))) _pollinginterval) (|(R/(Vpds-Vm)) _projectilespeed (/ (- (Math|Vector|VectorLength (- (.Location (Math|Transform|BreakTransform CurrentLocation)) (Variables|Default|GetDefenseOrigin))) (Math|Vector|VectorLength (- (.Location (Math|Transform|BreakTransform InitialLocation)) (Variables|Default|GetDefenseOrigin)))) _pollinginterval) (Math|Vector|VectorLength (- (.Location (Math|Transform|BreakTransform CurrentLocation)) (Variables|Default|GetDefenseOrigin)))))) (+ (* (/ (Math|Trig|Acos(Degrees) (/ (Math|Vector2D|DotProduct(2D) (Math|Vector2D|MakeVector2D (.X (Math|Vector|BreakVector (- (.Location (Math|Transform|BreakTransform InitialLocation)) (Variables|Default|GetDefenseOrigin)))) (.Z (Math|Vector|BreakVector (- (.Location (Math|Transform|BreakTransform InitialLocation)) (Variables|Default|GetDefenseOrigin))))) (Math|Vector2D|MakeVector2D (.X (Math|Vector|BreakVector (- (.Location (Math|Transform|BreakTransform CurrentLocation)) (Variables|Default|GetDefenseOrigin)))) (.Z (Math|Vector|BreakVector (- (.Location (Math|Transform|BreakTransform CurrentLocation)) (Variables|Default|GetDefenseOrigin)))))) (* (Math|Vector|VectorLengthXY (Math|Conversions|ToVector(Vector2D) (Math|Vector2D|MakeVector2D (.X (Math|Vector|BreakVector (- (.Location (Math|Transform|BreakTransform InitialLocation)) (Variables|Default|GetDefenseOrigin)))) (.Z (Math|Vector|BreakVector (- (.Location (Math|Transform|BreakTransform InitialLocation)) (Variables|Default|GetDefenseOrigin))))))) (Math|Vector|VectorLengthXY (Math|Conversions|ToVector(Vector2D) (Math|Vector2D|MakeVector2D (.X (Math|Vector|BreakVector (- (.Location (Math|Transform|BreakTransform CurrentLocation)) (Variables|Default|GetDefenseOrigin)))) (.Z (Math|Vector|BreakVector (- (.Location (Math|Transform|BreakTransform CurrentLocation)) (Variables|Default|GetDefenseOrigin)))))))))) (Variables|Default|GetPollingInterval)) (|(R/(Vpds-Vm)) _projectilespeed (/ (- (Math|Vector|VectorLength (- (.Location (Math|Transform|BreakTransform CurrentLocation)) (Variables|Default|GetDefenseOrigin))) (Math|Vector|VectorLength (- (.Location (Math|Transform|BreakTransform InitialLocation)) (Variables|Default|GetDefenseOrigin)))) _pollinginterval) (Math|Vector|VectorLength (- (.Location (Math|Transform|BreakTransform CurrentLocation)) (Variables|Default|GetDefenseOrigin))))) (* 1 (|(acos((z/norm))) (.Z (Math|Vector|BreakVector (- (.Location (Math|Transform|BreakTransform CurrentLocation)) (Variables|Default|GetDefenseOrigin)))) (Math|Vector|VectorLength (- (.Location (Math|Transform|BreakTransform CurrentLocation)) (Variables|Default|GetDefenseOrigin)))))) (|(ti*Vpds) (|(R/(Vpds-Vm)) _projectilespeed (/ (- (Math|Vector|VectorLength (- (.Location (Math|Transform|BreakTransform CurrentLocation)) (Variables|Default|GetDefenseOrigin))) (Math|Vector|VectorLength (- (.Location (Math|Transform|BreakTransform InitialLocation)) (Variables|Default|GetDefenseOrigin)))) _pollinginterval) (Math|Vector|VectorLength (- (.Location (Math|Transform|BreakTransform CurrentLocation)) (Variables|Default|GetDefenseOrigin)))) _projectilespeed)) (|(((sin(theta))*(sin(phi)))*R) (|(ti*Vpds) (|(R/(Vpds-Vm)) _projectilespeed (/ (- (Math|Vector|VectorLength (- (.Location (Math|Transform|BreakTransform CurrentLocation)) (Variables|Default|GetDefenseOrigin))) (Math|Vector|VectorLength (- (.Location (Math|Transform|BreakTransform InitialLocation)) (Variables|Default|GetDefenseOrigin)))) _pollinginterval) (Math|Vector|VectorLength (- (.Location (Math|Transform|BreakTransform CurrentLocation)) (Variables|Default|GetDefenseOrigin)))) _projectilespeed) (+ (Math|Trig|Atan2(Radians) (.Y (Math|Vector|BreakVector (- (.Location (Math|Transform|BreakTransform CurrentLocation)) (Variables|Default|GetDefenseOrigin)))) (.X (Math|Vector|BreakVector (- (.Location (Math|Transform|BreakTransform CurrentLocation)) (Variables|Default|GetDefenseOrigin))))) (* (/ (Math|Trig|Acos(Degrees) (/ (Math|Vector2D|DotProduct(2D) (Math|Vector2D|MakeVector2D (.X (Math|Vector|BreakVector (- (.Location (Math|Transform|BreakTransform InitialLocation)) (Variables|Default|GetDefenseOrigin)))) (.Y (Math|Vector|BreakVector (- (.Location (Math|Transform|BreakTransform InitialLocation)) (Variables|Default|GetDefenseOrigin))))) (Math|Vector2D|MakeVector2D (.X (Math|Vector|BreakVector (- (.Location (Math|Transform|BreakTransform CurrentLocation)) (Variables|Default|GetDefenseOrigin)))) (.Y (Math|Vector|BreakVector (- (.Location (Math|Transform|BreakTransform CurrentLocation)) (Variables|Default|GetDefenseOrigin)))))) (* (Math|Vector|VectorLengthXY (Math|Conversions|ToVector(Vector2D) (Math|Vector2D|MakeVector2D (.X (Math|Vector|BreakVector (- (.Location (Math|Transform|BreakTransform InitialLocation)) (Variables|Default|GetDefenseOrigin)))) (.Y (Math|Vector|BreakVector (- (.Location (Math|Transform|BreakTransform InitialLocation)) (Variables|Default|GetDefenseOrigin))))))) (Math|Vector|VectorLengthXY (Math|Conversions|ToVector(Vector2D) (Math|Vector2D|MakeVector2D (.X (Math|Vector|BreakVector (- (.Location (Math|Transform|BreakTransform CurrentLocation)) (Variables|Default|GetDefenseOrigin)))) (.Y (Math|Vector|BreakVector (- (.Location (Math|Transform|BreakTransform CurrentLocation)) (Variables|Default|GetDefenseOrigin)))))))))) _pollinginterval) (|(R/(Vpds-Vm)) _projectilespeed (/ (- (Math|Vector|VectorLength (- (.Location (Math|Transform|BreakTransform CurrentLocation)) (Variables|Default|GetDefenseOrigin))) (Math|Vector|VectorLength (- (.Location (Math|Transform|BreakTransform InitialLocation)) (Variables|Default|GetDefenseOrigin)))) _pollinginterval) (Math|Vector|VectorLength (- (.Location (Math|Transform|BreakTransform CurrentLocation)) (Variables|Default|GetDefenseOrigin)))))) (+ (* (/ (Math|Trig|Acos(Degrees) (/ (Math|Vector2D|DotProduct(2D) (Math|Vector2D|MakeVector2D (.X (Math|Vector|BreakVector (- (.Location (Math|Transform|BreakTransform InitialLocation)) (Variables|Default|GetDefenseOrigin)))) (.Z (Math|Vector|BreakVector (- (.Location (Math|Transform|BreakTransform InitialLocation)) (Variables|Default|GetDefenseOrigin))))) (Math|Vector2D|MakeVector2D (.X (Math|Vector|BreakVector (- (.Location (Math|Transform|BreakTransform CurrentLocation)) (Variables|Default|GetDefenseOrigin)))) (.Z (Math|Vector|BreakVector (- (.Location (Math|Transform|BreakTransform CurrentLocation)) (Variables|Default|GetDefenseOrigin)))))) (* (Math|Vector|VectorLengthXY (Math|Conversions|ToVector(Vector2D) (Math|Vector2D|MakeVector2D (.X (Math|Vector|BreakVector (- (.Location (Math|Transform|BreakTransform InitialLocation)) (Variables|Default|GetDefenseOrigin)))) (.Z (Math|Vector|BreakVector (- (.Location (Math|Transform|BreakTransform InitialLocation)) (Variables|Default|GetDefenseOrigin))))))) (Math|Vector|VectorLengthXY (Math|Conversions|ToVector(Vector2D) (Math|Vector2D|MakeVector2D (.X (Math|Vector|BreakVector (- (.Location (Math|Transform|BreakTransform CurrentLocation)) (Variables|Default|GetDefenseOrigin)))) (.Z (Math|Vector|BreakVector (- (.Location (Math|Transform|BreakTransform CurrentLocation)) (Variables|Default|GetDefenseOrigin)))))))))) (Variables|Default|GetPollingInterval)) (|(R/(Vpds-Vm)) _projectilespeed (/ (- (Math|Vector|VectorLength (- (.Location (Math|Transform|BreakTransform CurrentLocation)) (Variables|Default|GetDefenseOrigin))) (Math|Vector|VectorLength (- (.Location (Math|Transform|BreakTransform InitialLocation)) (Variables|Default|GetDefenseOrigin)))) _pollinginterval) (Math|Vector|VectorLength (- (.Location (Math|Transform|BreakTransform CurrentLocation)) (Variables|Default|GetDefenseOrigin))))) (* 1 (|(acos((z/norm))) (.Z (Math|Vector|BreakVector (- (.Location (Math|Transform|BreakTransform CurrentLocation)) (Variables|Default|GetDefenseOrigin)))) (Math|Vector|VectorLength (- (.Location (Math|Transform|BreakTransform CurrentLocation)) (Variables|Default|GetDefenseOrigin))))))) (|((cos(Phi))*R) (|(ti*Vpds) (|(R/(Vpds-Vm)) _projectilespeed (/ (- (Math|Vector|VectorLength (- (.Location (Math|Transform|BreakTransform CurrentLocation)) (Variables|Default|GetDefenseOrigin))) (Math|Vector|VectorLength (- (.Location (Math|Transform|BreakTransform InitialLocation)) (Variables|Default|GetDefenseOrigin)))) _pollinginterval) (Math|Vector|VectorLength (- (.Location (Math|Transform|BreakTransform CurrentLocation)) (Variables|Default|GetDefenseOrigin)))) _projectilespeed) (+ (* (/ (Math|Trig|Acos(Degrees) (/ (Math|Vector2D|DotProduct(2D) (Math|Vector2D|MakeVector2D (.X (Math|Vector|BreakVector (- (.Location (Math|Transform|BreakTransform InitialLocation)) (Variables|Default|GetDefenseOrigin)))) (.Z (Math|Vector|BreakVector (- (.Location (Math|Transform|BreakTransform InitialLocation)) (Variables|Default|GetDefenseOrigin))))) (Math|Vector2D|MakeVector2D (.X (Math|Vector|BreakVector (- (.Location (Math|Transform|BreakTransform CurrentLocation)) (Variables|Default|GetDefenseOrigin)))) (.Z (Math|Vector|BreakVector (- (.Location (Math|Transform|BreakTransform CurrentLocation)) (Variables|Default|GetDefenseOrigin)))))) (* (Math|Vector|VectorLengthXY (Math|Conversions|ToVector(Vector2D) (Math|Vector2D|MakeVector2D (.X (Math|Vector|BreakVector (- (.Location (Math|Transform|BreakTransform InitialLocation)) (Variables|Default|GetDefenseOrigin)))) (.Z (Math|Vector|BreakVector (- (.Location (Math|Transform|BreakTransform InitialLocation)) (Variables|Default|GetDefenseOrigin))))))) (Math|Vector|VectorLengthXY (Math|Conversions|ToVector(Vector2D) (Math|Vector2D|MakeVector2D (.X (Math|Vector|BreakVector (- (.Location (Math|Transform|BreakTransform CurrentLocation)) (Variables|Default|GetDefenseOrigin)))) (.Z (Math|Vector|BreakVector (- (.Location (Math|Transform|BreakTransform CurrentLocation)) (Variables|Default|GetDefenseOrigin)))))))))) (Variables|Default|GetPollingInterval)) (|(R/(Vpds-Vm)) _projectilespeed (/ (- (Math|Vector|VectorLength (- (.Location (Math|Transform|BreakTransform CurrentLocation)) (Variables|Default|GetDefenseOrigin))) (Math|Vector|VectorLength (- (.Location (Math|Transform|BreakTransform InitialLocation)) (Variables|Default|GetDefenseOrigin)))) _pollinginterval) (Math|Vector|VectorLength (- (.Location (Math|Transform|BreakTransform CurrentLocation)) (Variables|Default|GetDefenseOrigin))))) (* 1 (|(acos((z/norm))) (.Z (Math|Vector|BreakVector (- (.Location (Math|Transform|BreakTransform CurrentLocation)) (Variables|Default|GetDefenseOrigin)))) (Math|Vector|VectorLength (- (.Location (Math|Transform|BreakTransform CurrentLocation)) (Variables|Default|GetDefenseOrigin)))))))) (Variables|Default|GetDefenseOrigin))))

(fn TurnTurret
  (params (LocationToTurnTo :type Vector))
  (bind _returnvalue (Utilities|Time|GetWorldDeltaSeconds))
  (bind _returnvalue_2 (Utilities|Time|GetWorldDeltaSeconds))
  (bind _self self)
  (bind _turretrotator (Variables|Default|GetTurretRotator))
  (bind _turretrotator_2 (Variables|Default|GetTurretRotator))
  (bind _barrelrotator (Variables|Default|GetBarrelRotator))
  (bind _barrelrotator_2 (Variables|Default|GetBarrelRotator))
  (bind _turrettrackingspeed (Variables|Default|GetturretTrackingSpeed))
  (bind _turrettrackingspeed_2 (Variables|Default|GetturretTrackingSpeed))
  (bind _returnvalue_3 (Transformation|GetActorLocation _self))
  (bind _relativerotation (Variables|/Script/Engine.SceneComponent|GetRelativeRotation _turretrotator))
  (bind _relativerotation_2 (Variables|/Script/Engine.SceneComponent|GetRelativeRotation _barrelrotator_2))
  (bind (_x _y) (Math|Vector|BreakVector _returnvalue_3))
  (bind _returnvalue_4 (Math|Vector|MakeVector _x _y 345.0))
  (bind _returnvalue_5 (- LocationToTurnTo _returnvalue_4))
  (bind _returnvalue_6 (Math|Rotator|MakeRotfromX _returnvalue_5))
  (bind (_roll _pitch _yaw) (Math|Rotator|BreakRotator _returnvalue_6))
  (bind _returnvalue_7 (Math|Rotator|MakeRotator 0.0 0.0 _yaw))
  (bind _returnvalue_8 (* -1 _pitch))
  (bind _returnvalue_9 (Class|KismetMathLibrary|RInterptoConstant _relativerotation _returnvalue_7 _returnvalue _turrettrackingspeed))
  (bind _returnvalue_10 (Math|Rotator|MakeRotator _returnvalue_8 0.0 0.0))
  (bind _returnvalue_11 (Class|KismetMathLibrary|RInterptoConstant _relativerotation_2 _returnvalue_10 _returnvalue_2 _turrettrackingspeed_2))
  ;[1 1 1] Set rotations of the turret and barrels
  (Transformation|SetRelativeRotation _turretrotator_2 _returnvalue_9 false false)
  (Transformation|SetRelativeRotation _barrelrotator _returnvalue_11 false false)
  (return (Variables|/Script/Engine.SceneComponent|GetRelativeRotation _turretrotator_2) _returnvalue_9 (Variables|/Script/Engine.SceneComponent|GetRelativeRotation _barrelrotator) _returnvalue_11))

(fn FireTurret
  (params (BaseRotation :type Rotator) (TargetRotation :type Rotator) (BaseRotation2 :type Rotator) (TargetRotation2 :type Rotator)))

(fn TurnBarrels
  (params (targetLocation :type Vector))
  (bind _fireorigin1 (Variables|Default|GetFireOrigin1))
  (bind _fireorigin2 (Variables|Default|GetFireOrigin2))
  (bind _returnvalue (Transformation|GetWorldLocation _fireorigin2))
  (bind _returnvalue_2 (Transformation|GetWorldLocation _fireorigin1))
  (bind (_x _y) (Math|Vector|BreakVector _returnvalue))
  (bind (_x_2 _y_2) (Math|Vector|BreakVector _returnvalue_2))
  ;[1 1 1] Make rotator for the x (left-right) axis
  (Transformation|SetRelativeRotation (Variables|Default|GetFireOrigin1) (Math|Rotator|MakeRotator 0.0 0.0 (.Yaw (Math|Rotator|BreakRotator (Math|Rotator|MakeRotfromX (- targetLocation (Math|Vector|MakeVector _x_2 _y_2 0.0)))))) false false)
  (Transformation|SetRelativeRotation (Variables|Default|GetFireOrigin2) (Math|Rotator|MakeRotator 0.0 0.0 (.Yaw (Math|Rotator|BreakRotator (Math|Rotator|MakeRotfromX (- targetLocation (Math|Vector|MakeVector _x _y 0.0)))))) false false)
  (return))