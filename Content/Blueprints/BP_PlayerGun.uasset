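; BP_PlayerGun is the player's gun, with an ammo count that recharges and shows on the gun mesh as charge levels.
; Firing spawns a turret projectile at FireOrigin, tags it as a player gun shot and spends one bullet.
; A looping timer adds bullets with no upper limit, even during firing because it resets NotFiring before checking it.
; Tick clears seven named material slots, then refills one per seven bullets.
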(event Custom|fireBullet
  (if (> (Variables|Default|GetbulletCount) 0)
    (Variables|Default|SetnotFiring false)
    (bind _returnvalue (Game|SpawnActorfromClass "/Game/Blueprints/BP_TurretProjectile.BP_TurretProjectile_C" (Transformation|GetWorldTransform (Variables|Default|GetfireOrigin)) "AlwaysSpawn" 0 0))
    (Variables|/Game/Blueprints/BP_TurretProjectile.BP_TurretProjectile_C|SetbulletType _returnvalue "playerGun")
    (Variables|Default|SetbulletCount (- (Variables|Default|GetbulletCount) 1))))

(event Custom|replenishBullets
  (Variables|Default|SetnotFiring true)
  (if (Variables|Default|GetnotFiring)
    (Utilities|FlowControl|ForLoopwithBreak 0 0 :!label _label
      (:LoopBody
        (Variables|Default|SetbulletCount (+ (Variables|Default|GetbulletCount) 1))))
    (else
      (goto _label Break))))

(event EventBeginPlay
  (Utilities|Time|SetTimerbyEvent (delegate Custom|replenishBullets) 0.5 true))

(event EventTick
  (params (DeltaSeconds :type Float%20%28single-precision%29))
  (for _index (range 0 6)
    (Rendering|Material|SetMaterialbyName (Variables|Default|GetGunMesh) (Utilities|String|StringToName (Utilities|String|Append (Utilities|String|MakeLiteralString "chargeLevel") (Utilities|String|ToString(Integer) (- (Class|KismetSystemLibrary|MakeLiteralInteger 7) _index)))) "/Game/Assets/Materials/GunChargeEmpty.GunChargeEmpty"))
  (for _index_2 (range 1 (/ (Variables|Default|GetbulletCount) 7))
    (Rendering|Material|SetMaterialbyName (Variables|Default|GetGunMesh) (Utilities|String|StringToName (Utilities|String|Append (Utilities|String|MakeLiteralString "chargeLevel") (Utilities|String|ToString(Integer) _index_2))) "/Game/Assets/Materials/GunChargeFull.GunChargeFull")))

(fn ConstructionScript)